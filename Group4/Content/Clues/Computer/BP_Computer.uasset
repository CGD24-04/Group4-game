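; BP_Computer is an interactable computer actor among the game's clues, with a screen driven by a WBP_ComputerScreen widget.
; On BeginPlay it casts the user widget object of its UI component to that class and stores the reference.
; BeginInteract toggles the InteractionActive flag; nothing in this file reads the stored widget or acts further on the flag.
; An unconnected loop over PlayerText never runs.
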(event EventBeginPlay
  (bind _aswbp_computer_screen (Utilities|Casting|CastToWBP_ComputerScreen (UserInterface|GetUserWidgetObject (Variables|Default|GetUI))))
  (Variables|Default|SetAs%20WBP%20Computer%20Screen _aswbp_computer_screen))

(event Collision|EventActorBeginOverlap
  (params (OtherActor :type Actor%20Object%20Reference)))

(event EventTick
  (params (DeltaSeconds :type Float%20%28single-precision%29)))

(event EventBeginInteract
  (params (Player :type Actor%20Object%20Reference))
  (if (Variables|Default|GetInteraction%20Active)
    (Variables|Default|SetInteraction%20Active false)
    (else
      (Variables|Default|SetInteraction%20Active true))))

(fn ConstructionScript)