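; Actor component that lets the player inspect an interactable by rotating its tagged mesh in a close-up camera view.
; On BeginPlay it finds the owner's CineCamera and "InspectTarget" static mesh, printing warnings and invalidating the interaction if missing.
; BeginInteract toggles inspection, blending the view to the owner with tracking focus and input enabled, then back to the player.
; IA_Move rotates the mesh; ending resets rotation and notifies the player's AC_InteractionSystem.
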(event Input|EnhancedActionEvents|EnhancedInputActionIA_Move
  (params (ActionValue :type Vector%202D%20Structure) (ElapsedSeconds :type Float%20%28double-precision%29) (TriggeredSeconds :type Float%20%28double-precision%29) (InputAction :type Input%20Action%20Object%20Reference :default "/Game/ThirdPerson/Input/Actions/IA_Move.IA_Move"))
  (:Triggered
    (Transformation|AddWorldRotation (Variables|Default|GetActorToInspect) (Math|Rotator|MakeRotator 0.0 (.y ActionValue) (.x ActionValue)) false false)))

(event EventBeginInteract
  (params (Player :type Actor%20Object%20Reference))
  (bind _output_get (Variables|Default|SetInteractingActor Player))
  (if (Variables|Default|GetValid%20Interaction)
    (if (Variables|Default|GetIsInteracting)
      (CallFunction|EndInteractLogic)
      (else
        (CallFunction|BeginInteractLogic)))
    (else
      (Class|BPIPlayerInteract|EndInteract(Message) _output_get)
      (CallFunction|EndInteractLogic))))

(event EventStopInteract
  (params (Player :type Actor%20Object%20Reference)))

(event EventBeginPlay
  (bind _output_get (Variables|Default|SetOwner (Components|GetOwner)))
  (bind _output_get_2 (Variables|Default|SetInteractionCamera (Actor|GetComponentbyClass _output_get "/Script/CinematicCamera.CineCameraComponent")))
  (Utilities|IsValid _output_get_2
    (:Is%20Valid
      _)
    (:Is%20Not%20Valid
      (Development|PrintString "No CineCameraComponent on Interactable - Will not work!" true true "(R=1.000000,G=0.500000,B=0.000000,A=1.000000)" 1e+01)
      (Variables|Default|SetValid%20Interaction false)))
  (bind _output_get_3 (Variables|Default|SetActorToInspect (Utilities|Array|Get(acopy) (Actor|GetComponentsbyTag (Variables|Default|GetOwner) "/Script/Engine.StaticMeshComponent" "InspectTarget"))))
  (Utilities|IsValid _output_get_3
    (:Is%20Not%20Valid
      (Development|PrintString "No StaticMeshComponent Tagged with \"InspectTarget\" on Interactable - Will not work!" true true "(R=1.000000,G=0.500000,B=0.000000,A=1.000000)" 1e+01)
      (Variables|Default|SetValid%20Interaction false))))

(fn BeginInteractLogic
  (Game|Player|SetViewTargetwithBlend (Game|GetPlayerController 0) (Variables|Default|GetOwner) 1.0 "VTBlend_EaseInOut" 2.0 false)
  (Input|EnableInput (Variables|Default|GetOwner) (Game|GetPlayerController 0))
  (Variables|/Script/CinematicCamera.CineCameraComponent|SetFocusSettings (Variables|Default|GetInteractionCamera) (Utilities|Struct|MakeCameraFocusSettings "Tracking" 1e+05 (Utilities|Struct|MakeCameraTrackingFocusSettings (Utilities|ResolveSoftReference (Variables|Default|GetOwner)) "0.000000,0.000000,0.000000" false) false 8.0 0.0))
  (Variables|Default|SetIsInteracting true))

(fn EndInteractLogic
  (Game|Player|SetViewTargetwithBlend (Game|GetPlayerController 0) (Variables|Default|GetInteractingActor) 1.0 "VTBlend_EaseInOut" 2.0 false)
  (Transformation|SetWorldRotation (Variables|Default|GetActorToInspect) "0, 0, 0" false false)
  (Input|DisableInput (Variables|Default|GetOwner) (Game|GetPlayerController 0))
  (Class|BPIPlayerInteract|EndInteract(Message) (Actor|GetComponentbyClass (Variables|Default|GetInteractingActor) "/Game/DetectivePrototyp/AC_InteractionSystem.AC_InteractionSystem_C"))
  (Variables|Default|SetIsInteracting false))