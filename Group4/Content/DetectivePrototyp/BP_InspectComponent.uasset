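; BP_InspectComponent is an actor component that lets the player inspect and rotate an object through a dedicated camera.
; BeginInteract toggles the mode: entering blends the view to InteractionCamera, placed at CameraTransform with tracking focus on the owner, and enables owner input.
; IA_Move then adds pitch and yaw to ActorToInspect.
; Exiting restores the interacting actor's view, zeroes the object's rotation, disables input and notifies that actor's BP_InteractionSystem.
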(event Input|EnhancedActionEvents|EnhancedInputActionIA_Move
  (params (ActionValue :type Vector%202D%20Structure) (ElapsedSeconds :type Float%20%28double-precision%29) (TriggeredSeconds :type Float%20%28double-precision%29) (InputAction :type Input%20Action%20Object%20Reference :default "/Game/ThirdPerson/Input/Actions/IA_Move.IA_Move"))
  (:Triggered
    (Transformation|AddWorldRotation (Variables|Default|GetActorToInspect) (Math|Rotator|MakeRotator 0.0 (.y ActionValue) (.x ActionValue)) false false)))

(event EventBeginInteract
  (params (Player :type Actor%20Object%20Reference))
  (Variables|Default|SetInteractingActor Player)
  (if (Variables|Default|GetIsInteracting)
    (CallFunction|EndInteractLogic)
    (else
      (CallFunction|BeginInteractLogic))))

(event EventStopInteract
  (params (Player :type Actor%20Object%20Reference)))

(event EventBeginPlay
  (Variables|Default|SetOwner (Components|GetOwner)))

(fn BeginInteractLogic
  (bind _cameratransform (Variables|Default|GetCameraTransform))
  (Game|Player|SetViewTargetwithBlend (Game|GetPlayerController 0) (Variables|Default|GetInteractionCamera) 0.0 "VTBlend_Linear" 0.0 false)
  (Transformation|SetWorldLocationAndRotation (Variables|/Game/DetectivePrototyp/BP_InteractCam.BP_InteractCam_C|GetDefaultSceneRoot (Variables|Default|GetInteractionCamera)) (Transformation|GetWorldLocation _cameratransform) (Transformation|GetWorldRotation _cameratransform) false false)
  (Input|EnableInput (Variables|Default|GetOwner) (Game|GetPlayerController 0))
  (Variables|/Script/CinematicCamera.CineCameraComponent|SetFocusSettings (Variables|/Game/DetectivePrototyp/BP_InteractCam.BP_InteractCam_C|GetCineCamera (Variables|Default|GetInteractionCamera)) (Utilities|Struct|MakeCameraFocusSettings "Tracking" 1e+05 (Utilities|Struct|MakeCameraTrackingFocusSettings (Utilities|ResolveSoftReference (Components|GetOwner)) "0.000000,0.000000,0.000000" false) false 8.0 0.0))
  (Variables|Default|SetIsInteracting true))

(fn EndInteractLogic
  (Game|Player|SetViewTargetwithBlend (Game|GetPlayerController 0) (Variables|Default|GetInteractingActor) 0.0 "VTBlend_Linear" 0.0 false)
  (Transformation|SetWorldRotation (Variables|Default|GetActorToInspect) "0, 0, 0" false false)
  (Input|DisableInput (Variables|Default|GetOwner) (Game|GetPlayerController 0))
  (Class|BPIPlayerInteract|EndInteract(Message) (Actor|GetComponentbyClass (Variables|Default|GetInteractingActor) "/Game/DetectivePrototyp/BP_InteractionSystem.BP_InteractionSystem_C"))
  (Variables|Default|SetIsInteracting false))