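; Actor component that highlights its owning interactable while the player character overlaps it.
; On BeginPlay it caches every primitive component on the owner, binds their begin and end overlap events, and gives each a fixed custom depth stencil value.
; Player overlap toggles custom depth rendering on all cached components at once.
; Overlaps are not counted, so ending any single one turns the highlight off.
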(event Custom|OnComponentBeginOverlap_Event
  (params (OverlappedComponent :type Primitive%20Component%20Object%20Reference) (OtherActor :type Actor%20Object%20Reference) (OtherComp :type Primitive%20Component%20Object%20Reference) (OtherBodyIndex :type Integer) (bFromSweep :type Boolean) (SweepResult :type Hit%20Result%20Structure%20%28by%20ref%29))
  (if (== OtherActor (Game|GetPlayerCharacter 0))
    (for _array_element (Variables|Default|GetComponents)
      (Rendering|SetRenderCustomDepth _array_element true))))

(event Custom|OnComponentEndOverlap_Event
  (params (OverlappedComponent :type Primitive%20Component%20Object%20Reference) (OtherActor :type Actor%20Object%20Reference) (OtherComp :type Primitive%20Component%20Object%20Reference) (OtherBodyIndex :type Integer))
  (if (== OtherActor (Game|GetPlayerCharacter 0))
    (for _array_element (Variables|Default|GetComponents)
      (Rendering|SetRenderCustomDepth _array_element false))))

(event EventBeginPlay
  (for _array_element (Actor|GetComponentsByClass (Components|GetOwner) "/Script/Engine.PrimitiveComponent")
    (Collision|AssignOnComponentBeginOverlap _array_element (delegate Custom|OnComponentBeginOverlap_Event))
    (Collision|AssignOnComponentEndOverlap _array_element (delegate Custom|OnComponentEndOverlap_Event))
    (Rendering|SetCustomDepthStencilValue _array_element 150)
    (Utilities|Array|Add (Variables|Default|GetComponents) _array_element)))