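; BP_TorchPickup is an interactable world pickup that gives the player a torch in the detective prototype.
; On interact, it adds an unlimited-use Torch entry to the player's PlayerInventoryComponent, ends the interaction through AC_InteractionSystem, then destroys itself.
; A PathBlocking element is enabled on BeginPlay and disabled when the torch is taken, so the pickup gates a path.
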(event EventBeginPlay
  (Class|PathBlockingComponent|Enable (Variables|Default|GetPathBlocking)))

(event EventBeginInteract
  (params (Player :type Actor%20Object%20Reference))
  (bind _returnvalue (Actor|GetComponentbyClass Player "/Script/Group4.PlayerInventoryComponent"))
  (Utilities|IsValid _returnvalue
    (:Is%20Valid
      (Class|PlayerInventoryComponent|AddtoInventory _returnvalue (Utilities|Struct|MakeInventoryObjectData "Torch" false))
      (Class|BPIPlayerInteract|EndInteract(Message) (Actor|GetComponentbyClass Player "/Game/DetectivePrototyp/AC_InteractionSystem.AC_InteractionSystem_C"))
      (Class|PathBlockingComponent|Disable (Variables|Default|GetPathBlocking))
      (Actor|DestroyActor))))

(fn ConstructionScript)