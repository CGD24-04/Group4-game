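; BP_TestChild is a test interactable child Blueprint in the detective prototype that lets a player inspect its cube.
; On BeginPlay it hands the cube, a camera transform and the level's BP_InteractCam to its BPInspectComponent.
; BeginInteract calls the parent and the inspect component only if the player overlaps the actor.
; StopInteract forwards to both without that check.
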(event EventBeginInteract
  (params (Player :type Actor%20Object%20Reference))
  (for _array_element (Collision|GetOverlappingActors 0 :!class /Script/Engine.Actor)
    (if (== _array_element Player)
      (|CallParentFunction Player)
      (Default|BeginInteract (Variables|Default|GetBP_InspectComponent) Player))))

(event EventStopInteract
  (params (Player :type Actor%20Object%20Reference))
  (|CallParentFunction Player)
  (Default|StopInteract (Variables|Default|GetBP_InspectComponent) Player))

(event EventBeginPlay
  (bind _returnvalue (Actor|GetActorOfClass "/Game/DetectivePrototyp/BP_InteractCam.BP_InteractCam_C"))
  (Variables|/Game/DetectivePrototyp/BP_InspectComponent.BP_InspectComponent_C|SetInteractionCamera (Variables|Default|GetBP_InspectComponent) _returnvalue)
  (Variables|/Game/DetectivePrototyp/BP_InspectComponent.BP_InspectComponent_C|SetActorToInspect (Variables|Default|GetBP_InspectComponent) (Variables|Default|GetCube))
  (Variables|/Game/DetectivePrototyp/BP_InspectComponent.BP_InspectComponent_C|SetCameraTransform (Variables|Default|GetBP_InspectComponent) (Variables|Default|GetCamera%20transform)))

(fn ConstructionScript
  (|CallParentFunction))